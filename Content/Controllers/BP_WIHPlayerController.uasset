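; BP_WIHPlayerController is a player controller that updates the health bar in response to character begin, destroy and reach-goal calls.
; Each function casts the HUD to BP_HUD_DHV, calls CreateHUD, stores the returned widget in UIWBHUD and updates its health bar.
; CharacterBegin passes in the supplied health percent, while CharacterDestroy and CharacterReachGoal both set it to zero.
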(event EventBeginPlay)

(event EventTick
  (params (DeltaSeconds :type Float%20%28single-precision%29)))

(fn ConstructionScript)

(fn CharacterBegin
  (params (HealthPercent :type Float%20%28double-precision%29))
  (bind _asbp_hud_dhv (Utilities|Casting|CastToBP_HUD_DHV (HUD|GetHUD)))
  (bind _ui_wb_hud (Default|CreateHUD _asbp_hud_dhv))
  (bind _output_get (Variables|Default|SetUI%20WB%20HUD _ui_wb_hud))
  (Default|UpdateHealthBar _output_get HealthPercent))

(fn CharacterDestroy
  (bind _asbp_hud_dhv (Utilities|Casting|CastToBP_HUD_DHV (HUD|GetHUD)))
  (bind _ui_wb_hud (Default|CreateHUD _asbp_hud_dhv))
  (bind _output_get (Variables|Default|SetUI%20WB%20HUD _ui_wb_hud))
  (Default|UpdateHealthBar _output_get 0.0))

(fn CharacterReachGoal
  (bind _asbp_hud_dhv (Utilities|Casting|CastToBP_HUD_DHV (HUD|GetHUD)))
  (bind _ui_wb_hud (Default|CreateHUD _asbp_hud_dhv))
  (bind _output_get (Variables|Default|SetUI%20WB%20HUD _ui_wb_hud))
  (Default|UpdateHealthBar _output_get 0.0))