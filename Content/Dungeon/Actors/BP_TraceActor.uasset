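; BP_TraceActor is a debug test actor that traces ahead of itself and reports what it hits.
; Each Tick it runs a multi sphere trace for a single object type along its forward vector, using a math expression for the end point.
; For every blocking hit it draws a debug sphere at the impact point and prints the hit bone name.
; Prints for hit actor and component names are left disconnected.
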(event EventBeginPlay)

(event Collision|EventActorBeginOverlap
  (params (OtherActor :type Actor%20Object%20Reference)))

(event EventTick
  (params (DeltaSeconds :type Float%20%28single-precision%29))
  (bind _returnvalue (Transformation|GetActorLocation))
  (bind _outhits (Collision|MultiSphereTraceForObjects _returnvalue (|(ActorLocation+(ActorDirection*TraceLength)) _returnvalue (Transformation|GetActorForwardVector) 1e+03) 5e+01 (Utilities|Array|MakeArray "ObjectTypeQuery7") false 0 "ForOneFrame"))
  (for _array_element _outhits
    (if (.bBlockingHit (Collision|BreakHitResult _array_element))
      (Rendering|Debug|DrawDebugSphere (.ImpactPoint (Collision|BreakHitResult _array_element)) 1e+01 12 "(R=0.708333,G=0.708333,B=0.708333,A=1.000000)" -1.0 1.0)
      (Development|PrintString (Utilities|String|Append "Bone Name = " (Utilities|String|ToString(Name) (.HitBoneName (Collision|BreakHitResult _array_element)))) true true "(R=0.000000,G=0.660000,B=1.000000,A=1.000000)" -1.0))))

(fn ConstructionScript)