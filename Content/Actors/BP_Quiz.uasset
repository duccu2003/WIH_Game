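; BP_Quiz is an interactable actor that offers a pick prompt when the BP_DHV_Male character enters its capsule.
; Begin overlap shows a Pick widget, stores it in UIRef, sets the character's CanPick and passes "BP_Quiz" as its Item.
; End overlap removes a newly created Pick widget rather than UIRef, and leaves CanPick set.
; The node chain that opens the WB_QZ_01 widget is unconnected.
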(event OnComponentBeginOverlap(Capsule)
  (params (OverlappedComponent :type Primitive%20Component%20Object%20Reference) (OtherActor :type Actor%20Object%20Reference) (OtherComp :type Primitive%20Component%20Object%20Reference) (OtherBodyIndex :type Integer) (bFromSweep :type Boolean) (SweepResult :type Hit%20Result%20Structure%20%28by%20ref%29))
  (bind _asbp_dhv_male (Utilities|Casting|CastToBP_DHV_Male OtherActor))
  (bind _returnvalue (UserInterface|CreateWidget "/Game/UI/Widget/Pick.Pick_C"))
  (bind _output_get (Variables|Default|SetUI%20Ref _returnvalue))
  (UserInterface|Viewport|AddtoViewport _output_get 0)
  (Variables|/Game/Characters/BP_DHV_Male.BP_DHV_Male_C|SetCanPick _asbp_dhv_male true)
  (Variables|/Game/Characters/BP_DHV_Male.BP_DHV_Male_C|SetItem? _asbp_dhv_male "BP_Quiz"))

(event OnComponentEndOverlap(Capsule)
  (params (OverlappedComponent :type Primitive%20Component%20Object%20Reference) (OtherActor :type Actor%20Object%20Reference) (OtherComp :type Primitive%20Component%20Object%20Reference) (OtherBodyIndex :type Integer))
  (Utilities|Casting|CastToBP_DHV_Male OtherActor)
  (bind _returnvalue (UserInterface|CreateWidget "/Game/UI/Widget/Pick.Pick_C"))
  (Widget|RemovefromParent _returnvalue))

(fn ConstructionScript)