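; BP_HP_Dropping is a health pickup actor that heals a BP_DHV_Male character on contact.
; When its Box is overlapped, it adds a random integer amount to the character's BPHealthComponent health, clamped to HealthMax.
; It then passes the rolled, unclamped amount to the character's HealthBuffView and destroys itself.
; End overlap only casts, and a float-based random roll is left unconnected.
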(event OnComponentBeginOverlap(Box)
  (params (OverlappedComponent :type Primitive%20Component%20Object%20Reference) (OtherActor :type Actor%20Object%20Reference) (OtherComp :type Primitive%20Component%20Object%20Reference) (OtherBodyIndex :type Integer) (bFromSweep :type Boolean) (SweepResult :type Hit%20Result%20Structure%20%28by%20ref%29))
  (bind _asbp_dhv_male (Utilities|Casting|CastToBP_DHV_Male OtherActor))
  (bind _output_get (Variables|Default|SetHP_Count_Int (Math|Random|RandomIntegerinRange 10 100)))
  (Variables|/Game/Components/BP_HealthComponent.BP_HealthComponent_C|SetHealth (Variables|/Game/Characters/BP_DHV_Male.BP_DHV_Male_C|GetBP_HealthComponent _asbp_dhv_male) (Math|Float|Clamp(Float) (+ (Variables|/Game/Components/BP_HealthComponent.BP_HealthComponent_C|GetHealth (Variables|/Game/Characters/BP_DHV_Male.BP_DHV_Male_C|GetBP_HealthComponent _asbp_dhv_male)) _output_get) 0.0 (Variables|/Game/Components/BP_HealthComponent.BP_HealthComponent_C|GetHealth_Max (Variables|/Game/Characters/BP_DHV_Male.BP_DHV_Male_C|GetBP_HealthComponent _asbp_dhv_male))))
  (Default|HealthBuffView _asbp_dhv_male _output_get)
  (Actor|DestroyActor))

(event OnComponentEndOverlap(Box)
  (params (OverlappedComponent :type Primitive%20Component%20Object%20Reference) (OtherActor :type Actor%20Object%20Reference) (OtherComp :type Primitive%20Component%20Object%20Reference) (OtherBodyIndex :type Integer))
  (Utilities|Casting|CastToBP_DHV_Male OtherActor))

(event EventBeginPlay)

(event Collision|EventActorBeginOverlap
  (params (OtherActor :type Actor%20Object%20Reference)))

(event EventTick
  (params (DeltaSeconds :type Float%20%28single-precision%29)))

(fn ConstructionScript)