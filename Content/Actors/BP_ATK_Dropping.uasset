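; BP_ATK_Dropping is a pickup that grants an attack boost to the BP_DHV_Male character.
; On Box overlap with that character, it adds a random integer to the character's ATKCount, passes the amount to AttackBuffView, then destroys itself.
; The end-overlap handler only casts, and a float randomizer for ATKCount is left unconnected.
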(event OnComponentBeginOverlap(Box)
  (params (OverlappedComponent :type Primitive%20Component%20Object%20Reference) (OtherActor :type Actor%20Object%20Reference) (OtherComp :type Primitive%20Component%20Object%20Reference) (OtherBodyIndex :type Integer) (bFromSweep :type Boolean) (SweepResult :type Hit%20Result%20Structure%20%28by%20ref%29))
  (bind _asbp_dhv_male (Utilities|Casting|CastToBP_DHV_Male OtherActor))
  (bind _output_get (Variables|Default|SetATK_Count_Int (Math|Random|RandomIntegerinRange 10 50)))
  (Variables|/Game/Characters/BP_DHV_Male.BP_DHV_Male_C|SetATK_Count _asbp_dhv_male (+ (Variables|/Game/Characters/BP_DHV_Male.BP_DHV_Male_C|GetATK_Count _asbp_dhv_male) _output_get))
  (Default|AttackBuffView _asbp_dhv_male _output_get)
  (Actor|DestroyActor))

(event OnComponentEndOverlap(Box)
  (params (OverlappedComponent :type Primitive%20Component%20Object%20Reference) (OtherActor :type Actor%20Object%20Reference) (OtherComp :type Primitive%20Component%20Object%20Reference) (OtherBodyIndex :type Integer))
  (Utilities|Casting|CastToBP_DHV_Male OtherActor))

(event EventBeginPlay)

(event Collision|EventActorBeginOverlap
  (params (OtherActor :type Actor%20Object%20Reference)))

(event EventTick
  (params (DeltaSeconds :type Float%20%28single-precision%29)))

(fn ConstructionScript)