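; Enemy attack component that plays melee combo montages and deals damage to what the swings hit.
; Attack requests cycle through a montage array with a minion fallback, buffering input until the combo window opens.
; Damage handlers sphere-trace between left or right hand sockets and apply point damage once per actor until the hit list is cleared.
; Owner references come through BPI_Enemy_Attack; Q and R skill handlers are mostly stubs.
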(event EventBeginPlay)

(event EventTick
  (params (DeltaSeconds :type Float%20%28single-precision%29)))

(fn HandleBeginDoDamage
  ;[1 1 1] Handle Begin Do Damage
  (Utilities|Array|Clear (Variables|Default|GetAlreadyHittedActors)))

(fn HandleDoDamage
  (params (HandSide :type E_HandSide%20Enum :default "NewEnumerator0"))
  ;[1 1 1] Handle Do Damage
  (CallFunction|TraceHitDoDamage HandSide))

(fn HandleAttack)

(fn HandleQAttack
  (Variables|Default|SetisAttacking? false))

(fn HandleRAttack
  (Variables|Default|SetisAttacking? false))

(fn TraceHitDoDamage
  (params (HandSide :type E_HandSide%20Enum :default "NewEnumerator0"))
  (bind (_starthitlocation _endhitlocation) (CallFunction|HandSide HandSide))
  ;[0.1406 0.1406 0.1406] Hit Attack
  (bind _outhits (Collision|MultiSphereTraceForObjects _starthitlocation _endhitlocation (Variables|Default|GetTraceHitRadius) (Variables|Default|GetTraceObjectType) false 0 (Variables|Default|GetDraw%20Debug%20Type) true "(R=1.000000,G=0.000000,B=0.000000,A=1.000000)" "(R=0.000000,G=1.000000,B=0.000000,A=1.000000)" 2.0))
  (for _array_element _outhits
    ;;[1 0.1458 0.1458] Handle for each Hit Result
    (if (.bBlockingHit (Collision|BreakHitResult _array_element))
      (if (not (Utilities|Array|ContainsItem (Variables|Default|GetAlreadyHittedActors) (.HitActor (Collision|BreakHitResult _array_element))))
        (CallFunction|HandleHitActor _array_element)
        (Utilities|Array|Add (Variables|Default|GetAlreadyHittedActors) (.HitActor (Collision|BreakHitResult _array_element)))))))

(fn HandleHitActor
  (params (HitResult :type Hit%20Result%20Structure))
  (bind _returnvalue (Components|GetOwner))
  (bind _hitactor (Collision|BreakHitResult HitResult))
  (if (Utilities|DoesObjectImplementInterface _returnvalue "/Game/Interfaces/BPI_Enemy_Attack.BPI_Enemy_Attack_C")
    (bind _controllerreference (Class|BPIEnemyAttack|BPIGetControllerReference(Message) _returnvalue))
    (Game|Damage|ApplyPointDamage _hitactor (Variables|Default|GetAttackDamage) (Math|Vector|GetUnitDirection(Vector) (Transformation|GetActorLocation _returnvalue) (Transformation|GetActorLocation _hitactor)) HitResult _controllerreference _returnvalue)))

(fn RequestAttack
  (if (Utilities|DoesObjectImplementInterface (Components|GetOwner) "/Game/Interfaces/BPI_Enemy_Attack.BPI_Enemy_Attack_C")
    (if (or (not (Variables|Default|GetisAttacking?)) (Variables|Default|GetbCanCombo))
      (CallFunction|Attack)
      (else
        (Variables|Default|SetbisSavingAttack true)))))

(fn Attack
  (bind _correct_attack_montage (CallFunction|GetCorrectAttackMontage))
  (bind _returnvalue (Components|GetOwner))
  (if (Utilities|DoesObjectImplementInterface _returnvalue "/Game/Interfaces/BPI_Enemy_Attack.BPI_Enemy_Attack_C")
    (bind _charaterreference (Class|BPIEnemyAttack|BPIGetCharacterReference(Message) _returnvalue))
    (Utilities|IsValid _correct_attack_montage
      (:Is%20Valid
        (Animation|PlayAnimMontage _charaterreference _correct_attack_montage 1.0 "None")
        (Utilities|FlowControl|Sequence
          (:then_0
            (Variables|Default|SetisAttacking? true)
            (Variables|Default|SetbCanCombo false)
            (Variables|Default|SetAttackIndex (|(({8CA5D8E4-45DC-DEF1-4017-FDB3B820C8AF}+1)%AttackMontagesLength) (Utilities|Array|Length (Variables|Default|GetAttackMomtages)))))
          (:then_1
            (bind _mouthlocation (Class|BPIEnemyAttack|BPIGetMouthSocket(Message) _returnvalue :!label _label))
            (Audio|PlaySoundatLocation (Variables|Default|GetStartAttackSound) _mouthlocation "0, 0, 0" 1.0 1.0 0.0 "/Game/Audios/Attenuations/SA_Attack_Sound.SA_Attack_Sound" 0 0 0))))
      (:Is%20Not%20Valid
        (Animation|PlayAnimMontage _charaterreference "/Game/Characters/Minions/Animations/Melee/Montages/Attacks/AM_Minions_Attack_A.AM_Minions_Attack_A" 1.0 "None")
        (Utilities|FlowControl|Sequence
          (:then_0
            (goto _label))
          (:then_1
            (Variables|Default|SetisAttacking? true)
            (Variables|Default|SetbCanCombo false)))))))

(fn RequestRAttack
  (params (AnimRAttack :type Anim%20Montage%20Object%20Reference)))

(fn HandSide
  (params (HandSide :type E_HandSide%20Enum :default "NewEnumerator1"))
  (bind _returnvalue (Components|GetOwner))
  (if (Utilities|DoesObjectImplementInterface _returnvalue "/Game/Interfaces/BPI_Enemy_Attack.BPI_Enemy_Attack_C")
    (bind _skeletalmeshcomponentreference (Class|BPIEnemyAttack|BPIGetSkeletalMeshComponentReference(Message) _returnvalue))
    (switch Utilities|FlowControl|Switch|SwitchonE_HandSide HandSide
      (:NewEnumerator0
        (return (Transformation|GetSocketLocation _skeletalmeshcomponentreference (Variables|Default|GetRight_Hit_Start)) (Transformation|GetSocketLocation _skeletalmeshcomponentreference (Variables|Default|GetRight_Hit_End))))
      (:NewEnumerator1
        (return (Transformation|GetSocketLocation _skeletalmeshcomponentreference (Variables|Default|GetLeft_Hit_Start)) (Transformation|GetSocketLocation _skeletalmeshcomponentreference (Variables|Default|GetLeft_Hit_End)))))
    (else
      (return "0, 0, 0" "0, 0, 0"))))

(fn HandleEndAttack
  ;[1 1 1] Handle Attack
  (Variables|Default|SetisAttacking? false)
  (Variables|Default|SetbCanCombo false)
  (Variables|Default|SetbisSavingAttack false)
  (Variables|Default|SetAttackIndex 0))

(fn HandleCombo
  (Variables|Default|SetbCanCombo true)
  (if (Variables|Default|GetbisSavingAttack)
    (CallFunction|RequestAttack)
    (Variables|Default|SetbisSavingAttack false)))

(fn GetCorrectAttackMontage
  (return (Utilities|Array|Get(acopy) (Variables|Default|GetAttackMomtages) (Variables|Default|GetAttackIndex))))