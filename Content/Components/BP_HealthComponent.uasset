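; BP_HealthComponent is a component that tracks health for whatever actor owns it.
; GetHealthPercent returns Health as a fraction of HealthMax, and UpdateHealthByDamage subtracts damage from Health, clamped between zero and HealthMax.
; Both functions compute through Math Expression nodes, and the event graph holds no active logic.
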(event EventBeginPlay)

(event EventTick
  (params (DeltaSeconds :type Float%20%28single-precision%29)))

(fn GetHealthPercent
  (return (|({99C48A8C-49D3-E684-9633-13BC1EF786CB}/{F4760FEC-4C15-E0D6-8E9D-5C81599A02FA}))))

(fn UpdateHealthbyDamage
  (params (Damage :type Float%20%28double-precision%29))
  (Variables|Default|SetHealth (|(clamp(({99C48A8C-49D3-E684-9633-13BC1EF786CB}-Damage),0,{F4760FEC-4C15-E0D6-8E9D-5C81599A02FA})) Damage)))