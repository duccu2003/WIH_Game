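; AI controller for enemies that runs BT_Enemy on possession and tracks the player through AI Perception.
; A successful sense sets the see-player flag and target actor in the Blackboard, cancels any pending give-up timer and plays a cast sound at the stimulus location.
; Losing the stimulus starts a timer that clears both Blackboard values after GiveUpSeconds, so the chase persists briefly.
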(event OnTargetPerceptionUpdated(AIPerception)
  (params (Actor :type Actor%20Object%20Reference) (Stimulus :type AI%20Stimulus%20Structure))
  (bind (_age _expirationage _strength _stimuluslocation _receiverlocation _tag _bsuccessfullysensed) (Utilities|Struct|BreakAIStimulus Stimulus))
  (if _bsuccessfullysensed
    (CallFunction|HandleSeePlayer Actor _stimuluslocation)
    (else
      (CallFunction|HandleLoseSightPlayer))))

(event EventBeginPlay)

(event EventTick
  (params (DeltaSeconds :type Float%20%28single-precision%29)))

(event EventPossess
  (params (PossessedPawn :type Pawn%20Object%20Reference))
  (Variables|Default|SetPossessed%20Pawn PossessedPawn)
  (AI|RunBehaviorTree "/Game/AI/BT_Enemy.BT_Enemy"))

(fn ConstructionScript)

(fn HandleSeePlayer
  (params (Actor :type Actor%20Object%20Reference) (Center :type Vector))
  (Utilities|Time|ClearandInvalidateTimerbyHandle (Variables|Default|GetGiveUpTimer))
  (AI|Components|Blackboard|SetValueasBool (Variables|Default|GetBlackboard) (Variables|Default|GetbSeePlayer) true)
  (AI|Components|Blackboard|SetValueasObject (Variables|Default|GetBlackboard) (Variables|Default|GetPlayerActor) Actor)
  (Audio|PlaySoundatLocation "/Game/Audios/SoundCue/Cast/Enemy/SC_Enemy_Cast.SC_Enemy_Cast" Center "0, 0, 0" 1.0 1.0 0.0 0 0 0 0))

(fn HandleLoseSightPlayer
  (bind _returnvalue (Utilities|Time|SetTimerbyFunctionName 0 "GiveUpChasePlayer" (Variables|Default|GetGiveUpSeconds)))
  (Variables|Default|SetGiveUpTimer _returnvalue))

(fn GiveUpChasePlayer
  (AI|Components|Blackboard|SetValueasBool (Variables|Default|GetBlackboard) (Variables|Default|GetbSeePlayer) false)
  (AI|Components|Blackboard|SetValueasObject (Variables|Default|GetBlackboard) (Variables|Default|GetPlayerActor) 0))